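; VR training ZOLL defibrillator (AED) with an opening lid, attachable electrodes, flashing shock button and voice prompts.
; A staged state machine (Initialization, Analysis, Shock-Compressions) chains sound clips through audio-finished callbacks and per-clip delays, running stage tasks between clips.
; Attached electrodes start analysis; shock triggers the patient animation and compression prompts, looping to analysis until repetitions run out and the ambulance ending plays.
; A second speaker gives compression-depth feedback.
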(event OnDropped(HandleGrabComponent)
  (Utilities|FlowControl|Delay 0.8)
  (Development|SetHiddeninGame (Variables|Default|GetAEDFinal_Handle) true false)
  (Development|SetHiddeninGame (Variables|Default|GetAEDFinal_Number2) true false)
  (Collision|SetCollisionEnabled (Variables|/Game/Levels/AED/AED_Electrode1/AED_Electrode1_BP.AED_Electrode1_BP_C|GetAED_Electrode1 (Variables|Electrodes|GetUnusedElectrode1)) "QueryAndPhysics")
  (Collision|SetCollisionEnabled (Variables|/Game/Levels/AED/AED_Electrode2/AED_Electrode2_BP1.AED_Electrode2_BP1_C|GetAED_Electrode2 (Variables|Electrodes|GetUnusedElectrode2)) "QueryAndPhysics"))

(event Custom|Play%20Next%20Sound
  (params (Sounds :type Array%20of%20Sound%20Wave%20Object%20References) (Delays :type Array%20of%20Floats%20%28double-precision%29))
  (bind _aed_speaker (Variables|Default|GetAED_Speaker))
  (Variables|AEDAudio|SetCurrent%20Sound%20Clips Sounds)
  (if (< (Variables|AEDAudio|GetCurrentIndex) (Utilities|Array|Length Sounds))
    (Audio|Components|Audio|SetSound _aed_speaker (Utilities|Array|Get(acopy) (Variables|AEDAudio|GetCurrent%20Sound%20Clips) (Variables|AEDAudio|GetCurrentIndex)))
    (Audio|Components|Audio|Play _aed_speaker 0.0)
    (EventDispatchers|BindEventtoOnAudioFinished _aed_speaker (delegate Custom|Handle%20Sound%20Finished))
    (elif (Utilities|Enum|Equal(Enum) (Variables|AEDAudio|GetAED%20Stage) "NewEnumerator2")
      (CallFunction|PlayAEDPatientAnalysisAudio))))

(event Custom|Handle%20Sound%20Finished
  (Utilities|FlowControl|Delay (Utilities|Array|Get(acopy) (Variables|AEDAudio|GetCurrent%20Delays) (Variables|AEDAudio|GetCurrentIndex)))
  (switch Utilities|FlowControl|Switch|SwitchonEnum_AED_Stages (Variables|AEDAudio|GetAED%20Stage)
    (:NewEnumerator0
      (CallFunction|ExecuteInitializationStageTasks))
    (:NewEnumerator1
      (CallFunction|ExecuteAnalysisStageTasks))
    (:NewEnumerator2
      (CallFunction|ExecuteShockCompressionsStageTasks)))
  (CallFunction|PlayNextSound (Variables|AEDAudio|GetCurrent%20Sound%20Clips)))

(event Custom|End%20Experiment
  (bind _returnvalue (Actor|GetActorOfClass "/Game/BP_LevelSequenceManager.BP_LevelSequenceManager_C"))
  (Sequencer|Player|Play (Variables|/Script/LevelSequence.LevelSequenceActor|GetSequencePlayer (Variables|/Game/BP_LevelSequenceManager.BP_LevelSequenceManager_C|GetAmbulance%20Arriving%20LS _returnvalue)) :!class /Script/MovieScene.MovieSceneSequencePlayer)
  (EventDispatchers|BindEventtoOnFinished (Variables|/Script/LevelSequence.LevelSequenceActor|GetSequencePlayer (Variables|/Game/BP_LevelSequenceManager.BP_LevelSequenceManager_C|GetAmbulance%20Arriving%20LS _returnvalue)) (delegate Custom|Scene%20Fade%20Out)))

(event Custom|Evoke%20Delay
  (params (Delay%20in%20Seconds :type Float%20%28double-precision%29))
  ;[0.07619 0.1946 0.305 1 14] Custom Delay for non-Event Graph functions
  (Utilities|FlowControl|Delay Delay%20in%20Seconds))

(event Custom|Play%20Shock%20and%20Compressions%20Audio
  ;[0.5156 0.4824 0.1445 0.501 12] Called from VRPawn.OnComponentBeginOverlap_Event
  (Variables|Default|SetIsShockFlashing false)
  (Variables|AEDAudio|SetCurrentIndex 0)
  (Variables|AEDAudio|SetCC%20Rep%20Count (Variables|AEDAudio|GetCC%20Rhythm%20Reps))
  (bind _output_get (Variables|AEDAudio|SetCurrent%20Sound%20Clips (Variables|AEDAudio|GetSFX%20ShockAndCompressions)))
  (bind _output_get_2 (Variables|AEDAudio|SetCurrent%20Delays (Variables|AEDAudio|GetDelay%20ShockAndCompressions)))
  (Variables|AEDAudio|SetAED%20Stage "NewEnumerator2")
  (CallFunction|PlayNextSound _output_get _output_get_2))

(event Custom|Play%20AED%20Initialization%20Audio
  ;[0.5156 0.4824 0.1445 0.501 12] Called from WBP_AED_Container
  (Variables|AEDAudio|SetCurrentIndex 0)
  (bind _output_get (Variables|AEDAudio|SetCurrent%20Sound%20Clips (Variables|AEDAudio|GetSFX%20InitializeAED)))
  (bind _output_get_2 (Variables|AEDAudio|SetCurrent%20Delays (Variables|AEDAudio|GetDelays%20InitializeAED)))
  (Variables|AEDAudio|SetAED%20Stage "NewEnumerator0")
  (CallFunction|PlayNextSound _output_get _output_get_2))

(event Custom|Check%20Electrodes
  (if (CallFunction|AreBothElectrodesAttached)
    (CallFunction|PlayAEDPatientAnalysisAudio)))

(event Custom|Play%20AED%20Patient%20Analysis%20Audio
  ;[0.5156 0.4824 0.1445 0.501 12] Called by this.CheckElectrodes()
  (Variables|AEDAudio|SetCurrentIndex 0)
  (bind _output_get (Variables|AEDAudio|SetCurrent%20Sound%20Clips (Variables|AEDAudio|GetSFX%20AnalyzingPatient)))
  (bind _output_get_2 (Variables|AEDAudio|SetCurrent%20Delays (Variables|AEDAudio|GetDelays%20AnalyzingPatient)))
  (Variables|AEDAudio|SetAED%20Stage "NewEnumerator1")
  (CallFunction|PlayNextSound _output_get _output_get_2))

(event Custom|Play%20CC%20Feedback
  (params (DepthFlag :type Integer))
  (bind _aed_2ndspeaker (Variables|Default|GetAED_2ndSpeaker))
  (bind _aed_2ndspeaker_2 (Variables|Default|GetAED_2ndSpeaker))
  (if (CallFunction|AreBothElectrodesAttached)
    (switch int DepthFlag
      (:0
        (Audio|Components|Audio|SetSound _aed_2ndspeaker (Variables|AEDAudio|GetFeedback_GoodCompression))
        (Audio|Components|Audio|Play _aed_2ndspeaker 0.0)
        (Utilities|FlowControl|Delay 2.0))
      (:1
        (Audio|Components|Audio|SetSound _aed_2ndspeaker_2 (Variables|AEDAudio|GetFeedback_CompressHarder))
        (Audio|Components|Audio|Play _aed_2ndspeaker_2 0.0)
        (Utilities|FlowControl|Delay 2.0)))))

(event Custom|Open%20Lid
  ;[1 1 1] Open Lid Animation
  (Utilities|FlowControl|FlipFlop
    (:A
      (bind _lid_float (Timeline|OpenLidTimeline PlayFromStart)
        (:Update
          (Transformation|SetRelativeRotation (Variables|Default|GetLidPivot) (Math|Rotator|MakeRotator (Math|Float|Lerp 0.0 135.0 _lid_float) 0.0 0.0) false false)
          (Collision|SetCollisionEnabled (Variables|Default|GetAEDFinal_Handle) "QueryAndPhysics")
          (Collision|SetCollisionEnabled (Variables|Default|GetWidget) "NoCollision")
          (CallFunction|PlayAEDInitializationAudio))))
    (:B
      (Timeline|OpenLidTimeline Reverse))))

(event Custom|Flash%20Shock%20Button
  (if (Variables|Default|GetIsShockFlashing)
    (Rendering|Material|SetOverlayMaterial (Variables|Default|GetAEDFinal_Cylinder_001) "/Game/UI/M_Overlay_AEDShockBtn.M_Overlay_AEDShockBtn" :!class /Script/Engine.MeshComponent)
    (Utilities|FlowControl|Delay 0.3)
    (Rendering|Material|SetOverlayMaterial (Variables|Default|GetAEDFinal_Cylinder_001) 0 :!class /Script/Engine.MeshComponent)
    (Utilities|FlowControl|Delay 1.0)))

(event Custom|Scene%20Fade%20Out
  (bind _returnvalue (Actor|GetActorOfClass "/Game/BP_LevelSequenceManager.BP_LevelSequenceManager_C"))
  (Class|MovieSceneSequencePlayer|PlayReverse (Variables|/Script/LevelSequence.LevelSequenceActor|GetSequencePlayer (Variables|/Game/BP_LevelSequenceManager.BP_LevelSequenceManager_C|GetFadeInFadeOut%20LS _returnvalue))))

(event EventBeginPlay
  (Variables|AEDAudio|SetCurrent%20Sound%20Clips (Variables|AEDAudio|GetSFX%20InitializeAED))
  (Variables|AEDAudio|SetCurrent%20Delays (Variables|AEDAudio|GetDelays%20InitializeAED))
  (Variables|AEDAudio|SetAED%20Stage "NewEnumerator0")
  ;[1 1 1] Disable patch and lid collisions
  (bind _returnvalue (Actor|GetActorOfClass "/Game/Levels/AED/AED_Electrode1/AED_Electrode1_BP.AED_Electrode1_BP_C"))
  (bind _output_get (Variables|Electrodes|SetUnusedElectrode1 _returnvalue))
  (Collision|SetCollisionEnabled (Variables|/Game/Levels/AED/AED_Electrode1/AED_Electrode1_BP.AED_Electrode1_BP_C|GetAED_Electrode1 _output_get) "NoCollision")
  (bind _returnvalue_2 (Actor|GetActorOfClass "/Game/Levels/AED/AED_Electrode2/AED_Electrode2_BP1.AED_Electrode2_BP1_C"))
  (bind _output_get_2 (Variables|Electrodes|SetUnusedElectrode2 _returnvalue_2))
  (Collision|SetCollisionEnabled (Variables|/Game/Levels/AED/AED_Electrode2/AED_Electrode2_BP1.AED_Electrode2_BP1_C|GetAED_Electrode2 _output_get_2) "NoCollision")
  (Collision|SetCollisionEnabled (Variables|Default|GetAEDFinal_Handle) "NoCollision")
  ;[1 1 1] Disable Shock Button
  (Collision|SetCollisionEnabled (Variables|Default|GetAEDFinal_Cylinder_001) "NoCollision")
  (Collision|SetCollisionEnabled (Variables|Default|GetWidget) "NoCollision"))

(event Collision|EventActorBeginOverlap
  (params (OtherActor :type Actor%20Object%20Reference)))

(event EventTick
  (params (DeltaSeconds :type Float%20%28single-precision%29))
  (if (Utilities|Enum|Equal(Enum) (Variables|AEDAudio|GetAED%20Stage) "NewEnumerator1")
    (CallFunction|FlashShockButton)))

(event Input|KeyboardEvents|O
  (params (Key :type Key%20Structure :default "None"))
  (:Pressed
    (Transformation|SetRelativeRotation (Variables|Default|GetLidPivot) "0.000000,0.000000,135.000000" false false)))

(fn ConstructionScript)

(fn AreBothElectrodesAttached
  (return (and (Utilities|IsValid (Variables|Electrodes|GetSnappedElectrode1)) (Utilities|IsValid (Variables|Electrodes|GetSnappedElectrode2)))))

(fn ExecuteInitializationStageTasks
  (switch int 0
    (:Default
      (Math|Integer|IncrementInt (Variables|AEDAudio|GetCurrentIndex)
        (:%20%20
          (return))))))

(fn ExecuteAnalysisStageTasks
  (switch int (Variables|AEDAudio|GetCurrentIndex)
    (:0
      ;[1 1 1 1 14] check repetition of shock & cc
      (if (> (Variables|AEDAudio|GetShockRepetitions) 0)
        (Math|Integer|DecrementInt (Variables|AEDAudio|GetShockRepetitions)
          (:%20%20
            (Math|Integer|IncrementInt (Variables|AEDAudio|GetCurrentIndex)
              (:%20%20
                _))))
        (else
          (Variables|AEDAudio|SetCurrentIndex 4))))
    (:1
      (Math|Integer|IncrementInt (Variables|AEDAudio|GetCurrentIndex) :!label _label
        (:%20%20
          _)))
    (:2
      ;[1 1 1] Enable Shock Button
      (Collision|SetCollisionEnabled (Variables|Default|GetAEDFinal_Cylinder_001) "QueryAndPhysics")
      ;[1 1 1] TODO: flash SHOCK button
      (Variables|Default|SetIsShockFlashing true)
      (goto _label))
    (:3
      ;[1 1 1 1 12] Skip "iskua ei suositella" audio clip
      (Variables|AEDAudio|SetCurrentIndex (+ (Variables|AEDAudio|GetCurrentIndex) 2)))
    (:4
      (goto _label)))
  (return))

(fn ExecuteShockCompressionsStageTasks
  (bind _cc_rep_count (Variables|AEDAudio|GetCC%20Rep%20Count))
  (switch int (Variables|AEDAudio|GetCurrentIndex)
    (:Default
      (Math|Integer|IncrementInt (Variables|AEDAudio|GetCurrentIndex) :!label _label
        (:%20%20
          _)))
    (:0
      ;[1 1 1] Play Shock animation on Yuri
      (bind _returnvalue (Actor|GetActorOfClass "/Game/MetaHumans/Yuri/BP_Yuri.BP_Yuri_C"))
      (Default|PlayShockAnimation _returnvalue)
      (CallFunction|EvokeDelay 1.0)
      (goto _label))
    (:1
      (goto _label))
    (:2
      (goto _label))
    (:3
      (goto _label))
    (:4
      ;[1 1 1] Go back to Analysis stage
      (if (> _cc_rep_count 0)
        (Math|Integer|DecrementInt _cc_rep_count
          (:%20%20
            (goto _label)))
        (elif (> (Variables|AEDAudio|GetShockRepetitions) 0)
          (goto _label)
          (else
            (CallFunction|EndExperiment))))))
  (return))
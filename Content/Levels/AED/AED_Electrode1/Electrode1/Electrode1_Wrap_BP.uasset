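; Actor Blueprint for the first AED electrode pad, with a cable to the AED unit and a mesh that morphs via a Shrinkwrap target.
; On BeginPlay it attaches the cable end to the first AED_ZOLL_BP actor and looks up the BP_Yuri actor.
; Every Tick it copies Yuri's MorphValue onto the electrode mesh's Shrinkwrap morph target, so the wrap amount follows that character.
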(event EventBeginPlay
  (bind _outactors (Actor|GetAllActorsOfClass "/Game/Levels/AED/AED_ZOLL_BP.AED_ZOLL_BP_C"))
  (Class|CableComponent|SetAttachEndto (Variables|Default|GetCable) (Utilities|Array|Get(acopy) _outactors) "None" "None")
  (bind _outactors_2 (Actor|GetAllActorsOfClass "/Game/MetaHumans/Yuri/BP_Yuri.BP_Yuri_C")))

(event EventTick
  (params (DeltaSeconds :type Float%20%28single-precision%29))
  (bind _output_get (Variables|Default|Setmorph%20target%20wrap (Variables|/Game/MetaHumans/Yuri/BP_Yuri.BP_Yuri_C|GetMorph%20Value (Utilities|Array|Get(acopy) (stale EventBeginPlay _outactors_2)))))
  (Components|SkeletalMesh|SetMorphTarget (Variables|Default|GetElectrode1_Wrap) "Shrinkwrap" _output_get true))

(fn ConstructionScript)
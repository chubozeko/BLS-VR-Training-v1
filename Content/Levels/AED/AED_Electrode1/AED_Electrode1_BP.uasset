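; Grabbable first electrode patch for an AED, which snaps onto the chest of the patient (BP_Yuri).
; Each tick it tests collision between itself and the patient's Electrode1 spot.
; On contact it spawns a morph-target wrap electrode at the snapped position, registers it with AED_ZOLL_BP, triggers its electrode check and destroys itself.
; When dropped below zero height, it is put back at floor level keeping only yaw.
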(event OnGrabbed(GrabComponent))

(event OnDropped(GrabComponent)
  (bind _aed_electrode1 (Variables|Default|GetAED_Electrode1))
  (bind _returnvalue (Transformation|GetWorldLocation _aed_electrode1))
  (if (< (.z _returnvalue) 0.0)
    (Transformation|SetWorldLocationAndRotation _aed_electrode1 (Math|Vector|MakeVector (.x _returnvalue) (.y _returnvalue) 0.0) (Math|Rotator|MakeRotator 0.0 0.0 (.yaw (Transformation|GetWorldRotation _aed_electrode1))) false false)))

(event EventBeginPlay
  (bind _transform (Variables|Default|Gettransform))
  (bind _aed_electrode1 (Variables|Default|GetAED_Electrode1))
  (bind _returnvalue (Transformation|GetWorldTransform _aed_electrode1))
  (Variables|Default|SetIsSnappedToPatient false)
  (Collision|SetCollisionEnabled _aed_electrode1 "NoCollision")
  (bind _outactors (Actor|GetAllActorsOfClass "/Game/MetaHumans/Yuri/BP_Yuri.BP_Yuri_C"))
  ;[1 1 1] check collision for patch
  (if (not (== (Transformation|GetWorldTransform (Variables|/Game/MetaHumans/Yuri/BP_Yuri.BP_Yuri_C|GetElectrode1 (Utilities|Array|Get(acopy) _outactors))) _returnvalue))
    (if (not (stale _collided))
      (bind (_position _collided) (Class|PatchesCol|CheckCollision _returnvalue (Transformation|GetWorldTransform (Variables|/Game/MetaHumans/Yuri/BP_Yuri.BP_Yuri_C|GetElectrode1 (Utilities|Array|Get(acopy) _outactors)))))
      (if _collided
        ;[1 1 1] respawn patch on right position on chest with morph targets
        (Transformation|DetachFromActor "KeepRelative" "KeepRelative" "KeepRelative")
        (bind _returnvalue_2 (Game|SpawnActorfromClass "/Game/Levels/AED/AED_Electrode1/Electrode1/Electrode1_Wrap_BP.Electrode1_Wrap_BP_C" (Math|Transform|MakeTransform (.location _position) (.rotation _transform) (.scale _transform)) "AlwaysSpawn" "OverrideRootScale" 0 0))
        (Actor|Tick|SetActorTickEnabled _returnvalue_2 true)
        (Transformation|SetActorScale3D _returnvalue_2 "0.015000,0.015000,0.015000")
        (bind _returnvalue_3 (Actor|GetActorOfClass "/Game/Levels/AED/AED_ZOLL_BP.AED_ZOLL_BP_C"))
        (Variables|/Game/Levels/AED/AED_ZOLL_BP.AED_ZOLL_BP_C|SetSnappedElectrode1 _returnvalue_3 _returnvalue_2)
        (Default|CheckElectrodes _returnvalue_3)
        (Actor|DestroyActor)))))

(event EventTick
  (params (DeltaSeconds :type Float%20%28single-precision%29))
  (bind _transform (Variables|Default|Gettransform))
  (bind _aed_electrode1 (Variables|Default|GetAED_Electrode1))
  (bind _returnvalue (Transformation|GetWorldTransform _aed_electrode1))
  ;[1 1 1] check collision for patch
  (if (not (== (Transformation|GetWorldTransform (Variables|/Game/MetaHumans/Yuri/BP_Yuri.BP_Yuri_C|GetElectrode1 (Utilities|Array|Get(acopy) (stale EventBeginPlay _outactors)))) _returnvalue))
    (if (not (stale _collided))
      (bind (_position _collided) (Class|PatchesCol|CheckCollision _returnvalue (Transformation|GetWorldTransform (Variables|/Game/MetaHumans/Yuri/BP_Yuri.BP_Yuri_C|GetElectrode1 (Utilities|Array|Get(acopy) (stale EventBeginPlay _outactors))))))
      (if _collided
        ;[1 1 1] respawn patch on right position on chest with morph targets
        (Transformation|DetachFromActor "KeepRelative" "KeepRelative" "KeepRelative")
        (bind _returnvalue_2 (Game|SpawnActorfromClass "/Game/Levels/AED/AED_Electrode1/Electrode1/Electrode1_Wrap_BP.Electrode1_Wrap_BP_C" (Math|Transform|MakeTransform (.location _position) (.rotation _transform) (.scale _transform)) "AlwaysSpawn" "OverrideRootScale" 0 0))
        (Actor|Tick|SetActorTickEnabled _returnvalue_2 true)
        (Transformation|SetActorScale3D _returnvalue_2 "0.015000,0.015000,0.015000")
        (bind _returnvalue_3 (Actor|GetActorOfClass "/Game/Levels/AED/AED_ZOLL_BP.AED_ZOLL_BP_C"))
        (Variables|/Game/Levels/AED/AED_ZOLL_BP.AED_ZOLL_BP_C|SetSnappedElectrode1 _returnvalue_3 _returnvalue_2)
        (Default|CheckElectrodes _returnvalue_3)
        (Actor|DestroyActor)))))

(fn ConstructionScript)